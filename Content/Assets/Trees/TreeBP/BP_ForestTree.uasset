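; BP_ForestTree is a harvestable tree that turns into an inventory collectable after taking enough hits.
; Any hit on its StaticMesh, with no check on the source, starts a short Delay that also throttles repeat hits, then prints a debug message and decrements TreeHealth.
; At zero health it spawns a BP_Collectable at the mesh's location, configured as a stackable TreeBar item, and destroys itself.
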(event `self.ReceiveBeginPlay`
  (set `self.TreeHealth` 3))

(event `self.StaticMesh.OnComponentHit`
  (params (HitComponent :type "PrimitiveComponent Object Reference") (OtherActor :type "Actor Object Reference") (OtherComp :type "PrimitiveComponent Object Reference") (NormalImpulse :type "Vector Structure") (Hit :type "HitResult Structure (by ref)"))
  (bind _treehealth (`self.TreeHealth`))
  (bind (_returnvalue_x _returnvalue_y _returnvalue_z) (`KismetMathLibrary.BreakVector` (`SceneComponent.K2_GetComponentLocation` (`self.StaticMesh`))))
  (`KismetSystemLibrary.Delay` 0.3)
  (`KismetSystemLibrary.PrintString` "Hit!")
  (set `self.TreeHealth` (- _treehealth 1))
  (if (== _treehealth 0)
    (bind _output_get (set `self.TreeLocation` (`KismetMathLibrary.MakeVector` _returnvalue_x _returnvalue_y _returnvalue_z)))
    (`|SpawnActorFromClass` "/Game/Character/Inventory/BP_Collectable.BP_Collectable_C" (`KismetMathLibrary.Conv_VectorToTransform` _output_get) "Undefined" "MultiplyWithRoot" null (make `/Game/Character/Inventory/ST_Inventory` "TreeBar" "/Game/Assets/Trees/TreeBar.TreeBar" 1 10) null)
    (`self.K2_DestroyActor`)))

(fn `UserConstructionScript`)