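; BP_Collectable is a pickup actor that adds its item to the player's inventory when the player character overlaps its box.
; The overlap passes the pickup's Inventory data to the player's Comp_Inventory AddToInventory.
; On success it refreshes the grid of the first top-level W_Inventory widget found, destroys itself and prints a message.
; On failure it stays in the world and prints that the inventory is full.
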(event `self.Box.OnComponentBeginOverlap`
  (params (OverlappedComponent :type "PrimitiveComponent Object Reference") (OtherActor :type "Actor Object Reference") (OtherComp :type "PrimitiveComponent Object Reference") (OtherBodyIndex :type Integer) (bFromSweep :type Boolean) (SweepResult :type "HitResult Structure (by ref)"))
  (bind _asplayer_character_bp (cast `/Game/Character/PlayerCharacterBP` OtherActor))
  (bind _itemadded (`/Game/Inventory/Comp_Inventory.AddToInventory` (`self.GetComponentByClass` _asplayer_character_bp "/Game/Inventory/Comp_Inventory.Comp_Inventory_C") (`self.Inventory`)))
  (if _itemadded
    (bind _foundwidgets (`WidgetBlueprintLibrary.GetAllWidgetsOfClass` "/Game/Inventory/W_Inventory.W_Inventory_C"))
    (bind _output (`|GetArrayItem` _foundwidgets))
    (`/Engine/EditorBlueprintResources/StandardMacros.IsValid` _output
      (:`Is Valid`
        (`/Game/Inventory/W_Inventory.SetGrid` _output))
      (:`Is Not Valid`
        _))
    (`self.K2_DestroyActor`)
    (`KismetSystemLibrary.PrintString` "Item Collected")
    (else
      (`KismetSystemLibrary.PrintString` "Inventory Full"))))

(fn `UserConstructionScript`)