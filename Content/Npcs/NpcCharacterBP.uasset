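; NPC character Blueprint that shows an interaction prompt and opens dialogue, quest and shop widgets for the player.
; The ChkChar overlap shows or hides the Interact component, and on player exit also clears all widgets and restores game-only input.
; EventDialogue toggles the first-word dialogue widget, switching cursor and input mode and zeroing or restoring the NPC's own walk speed.
; Separate events add the quest and shop widgets to the viewport.
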(event `self.ReceiveBeginPlay`
  (`SceneComponent.SetHiddenInGame` (`self.CapsuleComponent`) true false))

(event `self.ChkChar.OnComponentBeginOverlap`
  (params (OverlappedComponent :type "PrimitiveComponent Object Reference") (OtherActor :type "Actor Object Reference") (OtherComp :type "PrimitiveComponent Object Reference") (OtherBodyIndex :type Integer) (bFromSweep :type Boolean) (SweepResult :type "HitResult Structure (by ref)"))
  (cast `/Game/Character/PlayerCharacterBP` OtherActor)
  (`SceneComponent.SetHiddenInGame` (`self.Interact`) false false))

(event `self.ChkChar.OnComponentEndOverlap`
  (params (OverlappedComponent :type "PrimitiveComponent Object Reference") (OtherActor :type "Actor Object Reference") (OtherComp :type "PrimitiveComponent Object Reference") (OtherBodyIndex :type Integer))
  (bind _returnvalue (`GameplayStatics.GetPlayerController` 0))
  (cast `/Game/Character/PlayerCharacterBP` OtherActor)
  (set `CharacterMovementComponent.MaxWalkSpeed` 600.0 (`self.CharacterMovement`))
  (`SceneComponent.SetHiddenInGame` (`self.Interact`) true false)
  (`WidgetLayoutLibrary.RemoveAllWidgets`)
  (set `PlayerController.bShowMouseCursor` false _returnvalue)
  (`WidgetBlueprintLibrary.SetInputMode_GameOnly` _returnvalue)
  (set `self.OpenWidget` false))

(event `/Game/Npcs/Dialogue.eventOnQuest`
  (bind _returnvalue (`|CreateWidget` "/Game/Npcs/WB_Quest.WB_Quest_C"))
  (`UserWidget.AddToViewport` _returnvalue 0))

(event `/Game/Npcs/Dialogue.eventOnShop`
  (bind _returnvalue (`|CreateWidget` "/Game/Npcs/WB_Shop.WB_Shop_C"))
  (`UserWidget.AddToViewport` _returnvalue 0))

(event `/Game/Npcs/Dialogue.eventDialogue`
  (bind _returnvalue (`GameplayStatics.GetPlayerController` 0))
  (bind _returnvalue_2 (`GameplayStatics.GetPlayerController` 0))
  (if (`self.OpenWidget`)
    (set `self.OpenWidget` false)
    (set `CharacterMovementComponent.MaxWalkSpeed` 600.0 (`self.CharacterMovement`))
    (`WidgetLayoutLibrary.RemoveAllWidgets`)
    (set `PlayerController.bShowMouseCursor` false _returnvalue_2)
    (`WidgetBlueprintLibrary.SetInputMode_GameOnly` _returnvalue_2)
    (else
      (set `self.OpenWidget` true)
      (`WidgetLayoutLibrary.RemoveAllWidgets`)
      (set `CharacterMovementComponent.MaxWalkSpeed` 0.0 (`self.CharacterMovement`))
      (bind _returnvalue_3 (`|CreateWidget` "/Game/Npcs/WB_FirstNpcWord.WB_FirstNpcWord_C"))
      (`UserWidget.AddToViewport` _returnvalue_3 0)
      (set `PlayerController.bShowMouseCursor` true _returnvalue)
      (`WidgetBlueprintLibrary.SetInputMode_GameAndUIEx` _returnvalue null))))

(fn `UserConstructionScript`)