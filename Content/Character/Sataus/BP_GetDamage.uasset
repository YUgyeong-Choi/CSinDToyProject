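; BP_GetDamage is a damage actor that hurts the player character when it overlaps the actor.
; On overlap, it stores the PlayerCharacterBP, sets the first flag in its Status struct and subtracts a fixed, clamped amount from the HP in WBStatus.
; After a short delay it clears that flag again, leaving the MP, Water and Hunger fields unchanged.
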(event `self.ReceiveActorBeginOverlap`
  (params (OtherActor :type "Actor Object Reference"))
  (bind _as_player_character_bp (`self.As Player Character BP`))
  (bind _wbstatus (`/Game/Character/PlayerCharacterBP.WBStatus` (`self.As Player Character BP`)))
  (bind (_status_hp _status_mp _status_water _status_hunger) (break `/Game/Character/Sataus/ST_Status` (`/Game/Character/PlayerCharacterBP.Status` _as_player_character_bp)))
  (bind _asplayer_character_bp (cast `/Game/Character/PlayerCharacterBP` OtherActor))
  (bind _output_get (set `self.As Player Character BP` _asplayer_character_bp))
  (bind (_status_hp_2 _status_mp_2 _status_water_2 _status_hunger_2) (break `/Game/Character/Sataus/ST_Status` (`/Game/Character/PlayerCharacterBP.Status` _output_get)))
  (set `/Game/Character/PlayerCharacterBP.Status` (make `/Game/Character/Sataus/ST_Status` true _status_mp_2 _status_water_2 _status_hunger_2) _output_get)
  (set `/Game/Character/Sataus/WB_Status.Hp` (`KismetMathLibrary.Clamp` (- (`/Game/Character/Sataus/WB_Status.Hp` _wbstatus) 100) 0 1000) _wbstatus)
  (`KismetSystemLibrary.Delay` 2.0)
  (set `/Game/Character/PlayerCharacterBP.Status` (make `/Game/Character/Sataus/ST_Status` false _status_mp _status_water _status_hunger) _as_player_character_bp))

(fn `UserConstructionScript`)